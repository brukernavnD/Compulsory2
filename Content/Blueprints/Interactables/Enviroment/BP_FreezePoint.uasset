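; BP_FreezePoint is an environment interactable that triggers the player's KillFreeze and destroys itself when an actor tagged Player overlaps its Box.
; Any hit on its Mesh calls CoolHook on the stored player reference.
; BeginPlay loops over actors found by class to set that reference, but the cast is disconnected from execution, so it is assigned None.
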(event OnComponentBeginOverlap(Box)
  (params (OverlappedComponent :type Primitive%20Component%20Object%20Reference) (OtherActor :type Actor%20Object%20Reference) (OtherComp :type Primitive%20Component%20Object%20Reference) (OtherBodyIndex :type Integer) (bFromSweep :type Boolean) (SweepResult :type Hit%20Result%20Structure%20%28by%20ref%29))
  (if (Actor|ActorHasTag OtherActor "Player")
    (CallFunction|KillFreeze (.As%20BP%20Player%20Character (Variables|Default|GetAs%20BP%20Player%20Character)))
    (Actor|DestroyActor)))

(event OnComponentHit(Mesh)
  (params (HitComponent :type Primitive%20Component%20Object%20Reference) (OtherActor :type Actor%20Object%20Reference) (OtherComp :type Primitive%20Component%20Object%20Reference) (NormalImpulse :type Vector :default "0, 0, 0") (Hit :type Hit%20Result%20Structure%20%28by%20ref%29))
  (CallFunction|CoolHook (.As%20BP%20Player%20Character (Variables|Default|GetAs%20BP%20Player%20Character))))

(event EventBeginPlay
  (bind _outactors (Actor|GetAllActorsOfClass 0))
  (for _array_element _outactors
    (Variables|Default|SetAs%20BP%20Player%20Character 0 _array_element)))

(fn ConstructionScript)