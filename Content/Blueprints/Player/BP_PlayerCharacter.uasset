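; Player character Blueprint that layers animation, effects, audio and HUD hooks onto grappling-hook movement.
; Grapple start and stop events drive hand-bone hiding, hook effects and pose montages picked by direction and hook time.
; Tick feeds velocity and rope reel rate into MetaSound parameters and material parameter collections, and applies hit-stop freezes through CustomTimeDilation.
; Slide input sets a placeholder dive flag; camera updates and objective overlap logic are disconnected.
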(event OnStartGrapple(GrappleComponent)
  (params (HitResult :type Hit%20Result%20Structure%20%28by%20ref%29))
  ;[0.3583 1 0] On Start Grapple
  (Utilities|FlowControl|Sequence
    (:then_0
      (Variables|Default|SetIs%20Grappling true))
    (:then_1
      (Variables|Default|SetGrapplePoint (.impactpoint HitResult))
      (Variables|Default|SetInitalGrappleDirectiom (Variables|/Script/Hilt.GrapplingComponent|GetGrappleDirection (Variables|Default|GetGrappleComponent))))
    (:then_2
      (Variables|Default|SetIsFrozen false))
    (:then_3
      (Components|SkinnedMesh|HideBonebyName (Variables|Character|GetMesh) "J_R_Wrist" "PBO_None"))
    (:then_4
      (Variables|Default|SetbCanActivateGrapple false)
      (Utilities|FlowControl|Delay 0.2)
      (Variables|Default|SetbCanActivateGrapple true))
    (:then_5
      (Class|AudioParameterControllerInterface|SetTriggerParameter (Variables|Default|GetMSS_Noises) "SwingSet"))
    (:then_6
      (Variables|Default|SetHookTIme 0.0))
    (:then_7
      (Variables|RopeLength|SetBufferRopeLength (Class|RopeComponent|GetRopeLength (Variables|Default|GetRopeComponent))))
    (:then_8
      (bind _hookreturn (Variables|Default|GetHookReturn)
        (:then
          (Components|DestroyComponent _hookreturn))
        (:else)))))

(event OnStopGrapple(GrappleComponent)
  ;[1 0.016 0] GrappleEnd
  (Utilities|FlowControl|Sequence
    (:then_0
      (Variables|Default|SetIs%20Grappling false))
    (:then_1
      (bind _spoolspark (Variables|Default|GetSpoolSpark)
        (:then
          (Components|DestroyComponent _spoolspark))
        (:else)))
    (:then_2
      (Components|SkinnedMesh|UnHideBonebyName (Variables|Character|GetMesh) "J_R_Wrist"))
    (:then_3
      (Audio|PlaySound2D 0 1.0 1.0 0.0 0 0))
    (:then_4
      (CallFunction|PostGrappleStart))
    (:then_5
      (Class|AudioParameterControllerInterface|SetTriggerParameter (Variables|Default|GetMSS_Noises) "SwingReset"))
    (:then_6
      (bind _returnvalue (Niagara|SpawnSystemAttached "/Game/Assets/VFX/GrapplingHook/NS_GrapplingEnd.NS_GrapplingEnd" (Variables|Character|GetMesh) "GrapplingHookSocket" "0, 0, 0" "0, 0, 0" "KeepRelativeOffset" false))
      (bind _output_get (Variables|Default|SetHookReturn _returnvalue))
      (Class|NiagaraComponent|SetVariablePosition _output_get "HookEnd" (Variables|Default|GetGrapplePoint)))))

(event Custom|CameraUpdates
  ;[0 0.3011 1] Camera Based Events (please Turn in to code later if possible thank you )(Also check construction script)
)

(event Custom|PostProcessUpdate
  (bind _returnvalue (Transformation|GetVelocity))
  (bind _cameraarm (Variables|Default|GetCameraArm))
  (bind _returnvalue_2 (Class|SpringArmComponent|GetTargetRotation _cameraarm))
  ;[0 0.3587 1] Post Process Updates
  (Utilities|FlowControl|Sequence
    (:then_0
      (Rendering|Material|SetScalarParameterValue "/Game/Assets/PostProcessing/MPC_Playerinfluencedmaterials.MPC_Playerinfluencedmaterials" "Speed" (Math|Float|MapRangeClamped (Math|Vector|VectorLength (Transformation|GetVelocity)) 0.0 4e+03 0.0 4.0) :!class /Script/Engine.KismetMaterialLibrary))
    (:then_1
      (Rendering|Material|SetVectorParameterValue "/Game/Assets/PostProcessing/MPC_Playerinfluencedmaterials.MPC_Playerinfluencedmaterials" "FullVelocity" (Utilities|Struct|MakeLinearColor (Math|Float|MapRangeClamped (.y (* (Math|Vector|GetRightVector _returnvalue_2) _returnvalue)) -5e+03 5e+03 1.0 0.0) (Math|Float|MapRangeClamped (.z (* (Transformation|GetVelocity) (Math|Vector|GetUpVector _returnvalue_2))) -6e+03 6e+03 0.0 1.0) (Math|Float|MapRangeClamped (.x (* _returnvalue (Math|Vector|GetForwardVector _returnvalue_2))) -1e+03 1e+03 0.0 1.0) 0.0) :!class /Script/Engine.KismetMaterialLibrary))))

(event Custom|KillFreeze
  ;[1 1 1] KillFreeze
  (Variables|Default|SetIsFrozen true)
  (Utilities|FlowControl|Delay 2.0)
  (Variables|Default|SetIsFrozen false))

(event Custom|FreezeCheck
  (if (Variables|Default|GetIsFrozen)
    (Variables|Default|SetCustomTimeDilation 0.0)
    (else
      (Variables|Default|SetCustomTimeDilation 1.0))))

(event Custom|CoolHook
  ;[1 1 1] Delay Effects
  (Utilities|FlowControl|Sequence
    (:then_0
      (Utilities|FlowControl|Delay 0.1)
      (Variables|Default|SetIsFrozen true)
      (Niagara|SpawnSystemAttached "/Game/Assets/VFX/GrapplingHook/MiscBonusGrapple/HandShot/NS_GrappleShotHand.NS_GrappleShotHand" (Variables|Character|GetMesh) "GrapplingHookSocket" "0, 0, 0" "0, 0, 0" "SnapToTargetIncludingScale" false)
      (Utilities|FlowControl|Delay 0.1)
      (Variables|Default|SetIsFrozen false))
    (:then_1
      (if (> (.Z (Math|Vector|BreakVector (Variables|/Script/Hilt.GrapplingComponent|GetGrappleDirection (Variables|Default|GetGrappleComponent)))) 0.0)
        (Animation|PlayAnimMontage (.OutItem (Utilities|Array|Random (Variables|Default|GetPose%20Below%20Anim))) 1.5 "None")
        (else
          (Animation|PlayAnimMontage (.OutItem (Utilities|Array|Random (Variables|Default|GetPose%20Above%20Anim))) 1.7 "None"))))))

(event Custom|CheckHookTime
  ;[0.3583 1 0] On Start Grapple
  (if (Variables|Default|GetIs%20Grappling)
    (bind _output_get (Variables|Default|SetHookTIme (+ (Variables|Default|GetHookTIme) (* 1.0 (Utilities|Time|GetWorldDeltaSeconds)))))))

(event Input|EnhancedActionEvents|EnhancedInputActionIA_PauseButton
  (params (ActionValue :type Boolean) (ElapsedSeconds :type Float%20%28double-precision%29) (TriggeredSeconds :type Float%20%28double-precision%29) (InputAction :type Input%20Action%20Object%20Reference :default "/Game/Blueprints/Player/Input/ActionInputs/IA_PauseButton.IA_PauseButton"))
  ;[1 1 1] Pause Game
  (bind _asbp_core_hud (Utilities|Casting|CastToBP_Core_HUD (HUD|GetHUD (Game|GetPlayerController 0))))
  (if (Game|IsGamePaused)
    (Default|ToggleCoreHUD _asbp_core_hud)
    (else
      (Default|TogglePause _asbp_core_hud))))

(event EventOnPlayerPickedUpAllObjectives
  ;[1 1 1] Activate on all objective taken
  (Default|ToggleScoreSceen (Variables|Default|GetCoreHud)))

(event EventBeginPlay
  (Utilities|FlowControl|Sequence
    (:then_0
      (bind _asbp_core_hud (Utilities|Casting|CastToBP_Core_HUD (HUD|GetHUD (Game|GetPlayerController 0))))
      (Variables|Default|SetCoreHud _asbp_core_hud))))

(event EventTick
  (params (DeltaSeconds :type Float%20%28single-precision%29))
  ;[0.2137 1 0] Event Tick
  (Utilities|FlowControl|Sequence
    (:then_2
      (CallFunction|StopPostGrappleMontage))
    (:then_3
      (CallFunction|PostProcessUpdate))
    (:then_4
      (CallFunction|FreezeCheck))
    (:then_5
      (CallFunction|WindNoise))
    (:then_6
      (Variables|Default|GetTimeSnapEffect
        (:then
          (CallFunction|SetAttractor))
        (:else)))
    (:then_7
      (CallFunction|SetSidetoSide))
    (:then_8
      (CallFunction|CheckHookTime))
    (:then_9
      (CallFunction|GrappleReel))))

(event Input|KeyboardEvents|1
  (params (Key :type Key%20Structure :default "None"))
  (:Pressed
    (Utilities|FlowControl|DoOnce false :!label _label
      (:Completed
        (for _array_element (Variables|/Script/Hilt.InventoryComponent|GetInventory (Variables|Default|GetInventoryComponent))
          (Development|PrintString (Utilities|GetObjectName (.Item (Utilities|Struct|BreakSlotStruct _array_element))))))))
  (:Released
    (goto _label Reset)))

(event Custom|WindNoise
  (Audio|Parameter|SetFloatParameter (Variables|Default|GetMSS_Noises) "Speed" (Math|Float|MapRangeClamped (Math|Vector|VectorLength (Transformation|GetVelocity)) 0.0 6e+03 0.0 1.0) :!class /Script/AudioExtensions.AudioParameterControllerInterface))

(event Custom|GrappleReel
  (bind _ropecomponent (Variables|Default|GetRopeComponent))
  (bind _returnvalue (Class|RopeComponent|GetRopeLength _ropecomponent))
  (bind _output_get (Variables|RopeLength|SetCurrentRopeLength (Math|Interpolation|FInterpTo (Variables|RopeLength|GetCurrentRopeLength) (* (- (Variables|RopeLength|GetBufferRopeLength) _returnvalue) (Utilities|Time|GetWorldDeltaSeconds)) (Utilities|Time|GetWorldDeltaSeconds) 4.0)))
  (Variables|RopeLength|SetRopeTension (Math|Interpolation|FInterpTo (Variables|RopeLength|GetCurrentRopeLength) (* (- (Variables|RopeLength|GetBufferRopeLength) _returnvalue) (Utilities|Time|GetWorldDeltaSeconds)) (Utilities|Time|GetWorldDeltaSeconds) 0.002))
  (Variables|RopeLength|SetBufferRopeLength _returnvalue)
  (Audio|Parameter|SetFloatParameter (Variables|Default|GetMSS_Noises) "ReelSpeed" (Variables|RopeLength|GetCurrentRopeLength) :!class /Script/AudioExtensions.AudioParameterControllerInterface)
  (Rendering|Material|SetScalarParameterValue "/Game/Assets/MaterialFunctions/MPC_RopeVariables.MPC_RopeVariables" "RopeTension" (Variables|RopeLength|GetRopeTension) :!class /Script/Engine.KismetMaterialLibrary))

(event Input|EnhancedActionEvents|EnhancedInputActionIA_StartSlide
  (params (ActionValue :type Boolean) (ElapsedSeconds :type Float%20%28double-precision%29) (TriggeredSeconds :type Float%20%28double-precision%29) (InputAction :type Input%20Action%20Object%20Reference :default "/Game/Blueprints/Player/Input/ActionInputs/IA_StartSlide.IA_StartSlide"))
  (if (and (AI|Components|NavMovement|IsFalling (Variables|Default|GetPlayerMovementComponent)) (not (Variables|Default|GetIs%20Grappling)))
    (Variables|Default|SetIsDiving true)
    (else
      (Variables|Default|SetIsDiving false))))

(event Input|EnhancedActionEvents|EnhancedInputActionIA_StopSlide
  (params (ActionValue :type Boolean) (ElapsedSeconds :type Float%20%28double-precision%29) (TriggeredSeconds :type Float%20%28double-precision%29) (InputAction :type Input%20Action%20Object%20Reference :default "/Game/Blueprints/Player/Input/ActionInputs/IA_StopSlide.IA_StopSlide"))
  (:Completed
    (Variables|Default|SetIsDiving false)))

(event Custom|PostGrappleStart
  (bind _mesh (Variables|Character|GetMesh))
  (bind _mesh_2 (Variables|Character|GetMesh))
  ;[1 1 1] Main Event
  (Utilities|FlowControl|Sequence
    (:then_0
      (if (>= (Variables|Default|GetHookTIme) 0.5)
        (if (> (Math|Float|Absolute(Float) (.Z (Math|Vector|BreakVector (Variables|/Script/Hilt.GrapplingComponent|GetGrappleDirection (Variables|Default|GetGrappleComponent))))) (Math|Float|Absolute(Float) (Variables|Default|GetGrappleSideToSideFloat)))
          (if (> (.Z (Math|Vector|BreakVector (Variables|/Script/Hilt.GrapplingComponent|GetGrappleDirection (Variables|Default|GetGrappleComponent)))) 0.0)
            (Animation|Montage|PlayMontage _mesh_2 (.OutItem (Utilities|Array|Random (Variables|Default|GetPose%20End%20Below%20Anim)))
              (:then
                (Variables|Default|SetPostGrappleMontage true))
              (:OnCompleted
                (Variables|Default|SetPostGrappleMontage false :!label _label))
              (:OnInterrupted
                (goto _label)))
            (else
              (Animation|Montage|PlayMontage _mesh_2 (.OutItem (Utilities|Array|Random (Variables|Default|GetPose%20End%20Above%20Anim)))
                (:then
                  (Variables|Default|SetPostGrappleMontage true))
                (:OnCompleted
                  (Variables|Default|SetPostGrappleMontage false :!label _label_2))
                (:OnInterrupted
                  (goto _label_2)))))
          (elif (>= (Variables|Default|GetGrappleSideToSideFloat) 0.0)
            (Animation|Montage|PlayMontage _mesh (.OutItem (Utilities|Array|Random (Variables|Default|GetPose%20End%20Right%20Anim))) 0.8
              (:then
                (Variables|Default|SetPostGrappleMontage true))
              (:OnCompleted
                (Variables|Default|SetPostGrappleMontage false :!label _label_3))
              (:OnInterrupted
                (goto _label_3)))
            (else
              (Animation|Montage|PlayMontage _mesh (.OutItem (Utilities|Array|Random (Variables|Default|GetPose%20End%20Left%20Anim)))
                (:then
                  (Variables|Default|SetPostGrappleMontage true))
                (:OnCompleted
                  (Variables|Default|SetPostGrappleMontage false :!label _label_4))
                (:OnInterrupted
                  (goto _label_4))))))))))

(event Custom|SetSideToSide
  ;[1 1 1] Side By Side Write
  (if (Variables|/Script/Hilt.GrapplingComponent|GetbIsGrappling (Variables|Default|GetGrappleComponent))
    (Variables|Default|SetGrappleSideToSideFloat (Math|Float|MapRangeClamped (Math|Rotator|NormalizeAxis (.yaw (Math|Rotator|Delta(Rotator) (Math|Rotator|FindRelativeLookatRotation (Math|Transform|MakeTransform (.location (Transformation|GetActorTransform)) "0, 0, 0" "1.000000,1.000000,1.000000") (Variables|Default|GetGrapplePoint)) (Math|Conversions|RotationFromXVector (Transformation|GetVelocity))))) -1.8e+02 1.8e+02 -1.0 1.0))))

(event Custom|StopPostGrappleMontage
  (bind _mesh (Variables|Character|GetMesh))
  (bind _returnvalue (Components|SkeletalMesh|GetAnimInstance _mesh))
  ;[1 1 1] StopGrapple
  (if (and (Variables|Default|GetPostGrappleMontage) (!= (AI|Components|NavMovement|IsFalling (Variables|Character|GetCharacterMovement)) true))
    (Animation|Montage|MontageSetPlayRate _returnvalue (Animation|Montage|GetCurrentActiveMontage _returnvalue) 1e+01)))

(event OnComponentBeginOverlap(CapsuleComponent)
  (params (OverlappedComponent :type Primitive%20Component%20Object%20Reference) (OtherActor :type Actor%20Object%20Reference) (OtherComp :type Primitive%20Component%20Object%20Reference) (OtherBodyIndex :type Integer) (bFromSweep :type Boolean) (SweepResult :type Hit%20Result%20Structure%20%28by%20ref%29)))

(event Custom|SetAttractor
  (Class|NiagaraComponent|SetVariablePosition (Variables|Default|GetTimeSnapEffect) "PlayerPos" (Transformation|GetActorLocation)))

(fn ConstructionScript
  (Utilities|FlowControl|Sequence
    (:then_0
      ;[0 0.2738 1] Camera Construction
      (Utilities|FlowControl|Sequence
        (:then_0
          (Variables|/Script/Engine.SpringArmComponent|SetTargetArmLength (Variables|Default|GetCameraArm) (Variables|Camera|GetCameraArmBaseLength)))
        (:then_1
          (Transformation|SetRelativeLocation (Variables|Default|GetCameraArm) (Variables|Camera|GetCameraArmBaseTransform) false false))))))